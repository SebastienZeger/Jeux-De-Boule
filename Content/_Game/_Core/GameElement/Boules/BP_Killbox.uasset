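; BP_Killbox is a trigger volume that destroys any actor entering it and penalizes the player's score.
; On Box begin overlap it destroys the other actor with no class filter, then casts the game mode to BP_GameMode.
; It prints a French taunt and, unless Score is already zero, decrements it and prints the new value.
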(event `self.Box.OnComponentBeginOverlap`
  (params (OverlappedComponent :type "PrimitiveComponent Object Reference") (OtherActor :type "Actor Object Reference") (OtherComp :type "PrimitiveComponent Object Reference") (OtherBodyIndex :type Integer) (bFromSweep :type Boolean) (SweepResult :type "HitResult Structure (by ref)"))
  (`self.K2_DestroyActor` OtherActor)
  (bind _asbp_game_mode (cast `/Game/_Game/_Core/GameElement/BP_GameMode` (`GameplayStatics.GetGameMode`)))
  (`|ExecutionSequence`
    (:`then_0`
      (`KismetSystemLibrary.PrintString` "Tu es NUL"))
    (:`then_1`
      (bind _score (`/Game/_Game/_Core/GameElement/BP_GameMode.Score` _asbp_game_mode))
      (if (not (== _score 0))
        (bind _result (`/Engine/EditorBlueprintResources/StandardMacros.DecrementInt` _score)
          (:`  `
            (`KismetSystemLibrary.PrintString` (`KismetStringLibrary.Conv_IntToString` _result))))))))

(fn `UserConstructionScript`)