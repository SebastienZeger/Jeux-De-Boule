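; BP_Filter is a color filter game element that repaints "Ball"-tagged actors overlapping its Box to match its Color, unless they are already black.
; White and Black filters tint their Cube at BeginPlay and lock color changes.
; Clicking a changeable filter's Cube opens WBP_ColorFilter with a reference to the filter and shows the mouse cursor.
; A helper, f_CheckColor, maps materials to StateColor but is not called here.
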(event `self.Box.OnComponentBeginOverlap`
  (params (OverlappedComponent :type "PrimitiveComponent Object Reference") (OtherActor :type "Actor Object Reference") (OtherComp :type "PrimitiveComponent Object Reference") (OtherBodyIndex :type Integer) (bFromSweep :type Boolean) (SweepResult :type "HitResult Structure (by ref)"))
  (bind _overlapedball (`self.OverlapedBall`))
  (if (`self.ActorHasTag` OtherActor "Ball")
    (set `self.OverlapedBall` OtherComp)
    (if (not (== (`PrimitiveComponent.GetMaterial` OtherComp 0) "/Game/_Game/Material/M_Black.M_Black"))
      (switch `string` (`self.Color`)
        (:`Blue`
          (`PrimitiveComponent.SetMaterial` _overlapedball 0 "/Game/_Game/Material/M_Blue.M_Blue"))
        (:`Red`
          (`PrimitiveComponent.SetMaterial` _overlapedball 0 "/Game/_Game/Material/M_Red.M_Red"))
        (:`Yellow`
          (`PrimitiveComponent.SetMaterial` _overlapedball 0 "/Game/_Game/Material/M_Yellow.M_Yellow"))
        (:`White`
          (`PrimitiveComponent.SetMaterial` _overlapedball 0 "/Game/_Game/Material/M_White.M_White"))
        (:`Black`
          (`PrimitiveComponent.SetMaterial` _overlapedball 0 "/Game/_Game/Material/M_Black.M_Black"))))))

(event `self.ReceiveBeginPlay`
  (bind _cube (`self.Cube`))
  (switch `string` (`self.Color`)
    (:`White`
      (`PrimitiveComponent.SetMaterial` _cube 0 "/Game/_Game/Material/M_White.M_White")
      (set `self.CanChangeColor` false))
    (:`Black`
      (`PrimitiveComponent.SetMaterial` _cube 0 "/Game/_Game/Material/M_Black.M_Black")
      (set `self.CanChangeColor` false))))

(event `self.Cube.OnClicked`
  (params (TouchedComponent :type "PrimitiveComponent Object Reference") (ButtonPressed :type "Key Structure"))
  (if (`self.CanChangeColor`)
    (set `self.Touched Component_0` TouchedComponent)
    (bind _returnvalue (`|CreateWidget` "/Game/_Game/_Core/GameElement/WBP_ColorFilter.WBP_ColorFilter_C"))
    (`UserWidget.AddToViewport` _returnvalue 0)
    (set `/Game/_Game/_Core/GameElement/WBP_ColorFilter.Filter` self _returnvalue)
    (set `PlayerController.bShowMouseCursor` true (`GameplayStatics.GetPlayerController` 0))))

(event `InputTouch`
  (params (Location :type "Vector Structure") (FingerIndex :type "ETouchIndex Enum")))

(fn `f_CheckColor`
  (params (Material :type "MaterialInterface Object Reference"))
  (if (== Material "/Game/_Game/Material/M_Blue.M_Blue")
    (set `self.StateColor` "NewEnumerator2")
    (elif (== Material "/Game/_Game/Material/M_Yellow.M_Yellow")
      (set `self.StateColor` "NewEnumerator1")
      (elif (== Material "/Game/_Game/Material/M_Red.M_Red")
        (set `self.StateColor` "NewEnumerator0")
        (elif (== Material "/Game/_Game/Material/M_Orange.M_Orange")
          (set `self.StateColor` "NewEnumerator3")
          (elif (== Material "/Game/_Game/Material/M_Green.M_Green")
            (set `self.StateColor` "NewEnumerator4")
            (elif (== Material "/Game/_Game/Material/M_Purple.M_Purple")
              (set `self.StateColor` "NewEnumerator5")
              (elif (== Material "/Game/_Game/Material/M_White.M_White")
                (set `self.StateColor` "NewEnumerator6")
                (elif (== Material "/Game/_Game/Material/M_Black.M_Black")
                  (set `self.StateColor` "NewEnumerator7"))))))))))

(fn `UserConstructionScript`)