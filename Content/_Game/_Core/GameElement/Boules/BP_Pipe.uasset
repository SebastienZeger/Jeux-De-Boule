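; BP_Pipe is a moving ball dispenser that releases stone balls based on how long the player holds IA_Spawn.
; The construction script sets InterpToMovement to travel between StartLocation and EndLocation over Duration.
; Holding the input opens a gate that lets a looping timer increment BallsToSpawn.
; On release, the gate closes, a loop spawns BP_Boule_Pierre actors at the Arrow for that count, and the count resets.
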(event `self.ReceiveBeginPlay`
  (`|ExecutionSequence`
    (:`then_0`
      (`self.BallSpawnTimer`))))

(event `SpawnActor`)

(event `BallSpawnTimer`
  (`KismetSystemLibrary.K2_SetTimerDelegate` (delegate `BallSpawn`) 0.1 true))

(event `BallSpawn`
  (`/Engine/EditorBlueprintResources/StandardMacros.Gate` true :!label _label
    (:`Exit`
      (bind _result (`/Engine/EditorBlueprintResources/StandardMacros.IncrementInt` (`self.BallsToSpawn`))
        (:`  `
          (set `self.BallsToSpawn` _result))))))

(event `EnhancedInput|/Game/_Game/_Core/GameElement/Inputs/IA_Spawn`
  (params (ActionValue :type Boolean) (ElapsedSeconds :type "Float (double-precision)") (TriggeredSeconds :type "Float (double-precision)") (InputAction :type "InputAction Object Reference" :default "/Game/_Game/_Core/GameElement/Inputs/IA_Spawn.IA_Spawn"))
  (:`Ongoing`
    (goto _label :!via `Open`))
  (:`Completed`
    (`|ExecutionSequence`
      (:`then_0`
        (goto _label :!via `Close`))
      (:`then_1`
        (for _ (`|MakeArray` (`self.BallsToSpawn`))
          (`|SpawnActorFromClass` "/Game/_Game/_Core/GameElement/Boules/BP_Boule_Pierre.BP_Boule_Pierre_C" (`KismetMathLibrary.Conv_VectorToTransform` (`SceneComponent.K2_GetComponentLocation` (`self.Arrow`))) "Undefined" "MultiplyWithRoot" null null)
          (`KismetSystemLibrary.Delay` 0.1))
        (set `self.BallsToSpawn` 0)))))

(fn `UserConstructionScript`
  (bind _interptomovement (`self.InterpToMovement`))
  (set `InterpToMovementComponent.ControlPoints` (`|MakeArray` (make `InterpControlPoint` (`self.StartLocation`)) (make `InterpControlPoint` (`self.EndLocation`))) _interptomovement)
  (set `InterpToMovementComponent.Duration` (`self.Duration`) _interptomovement))