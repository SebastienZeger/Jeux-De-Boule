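; BP_PipeMenu is a moving pipe, apparently for the menu, that repeatedly spawns BP_Ball actors with an exit sound.
; The construction script feeds StartLocation, EndLocation and Duration into InterpToMovement as a relative two-point path.
; At BeginPlay a looping timer takes one random sub-second interval, so each instance keeps a fixed spawn rate.
; Each tick of that timer spawns a ball at the SpawnerVolume's location.
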(event `self.ReceiveBeginPlay`
  (`self.BallSpawnTimer`))

(event `BallSpawnTimer`
  (`KismetSystemLibrary.K2_SetTimerDelegate` (delegate `BallSpawn`) (`KismetMathLibrary.RandomFloatInRange` 0.1 1.0) true))

(event `BallSpawn`
  (`|SpawnActorFromClass` "/Game/_Game/_Core/GameElement/BP_Ball.BP_Ball_C" (`KismetMathLibrary.Conv_VectorToTransform` (`SceneComponent.K2_GetComponentLocation` (`self.SpawnerVolume`))) "Undefined" "MultiplyWithRoot" null null)
  (`GameplayStatics.SpawnSound2D` "/Game/Sounds/Pipe_Exit_Cue.Pipe_Exit_Cue" 0.3 1.0 0.0 null))

(fn `UserConstructionScript`
  (bind _interptomovement (`self.InterpToMovement`))
  (set `InterpToMovementComponent.ControlPoints` (`|MakeArray` (make `InterpControlPoint` (`self.StartLocation`)) (make `InterpControlPoint` (`self.EndLocation`))) _interptomovement)
  (set `InterpToMovementComponent.Duration` (`self.Duration`) _interptomovement))