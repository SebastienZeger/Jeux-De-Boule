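; BP_Pipe is a ball-dispensing pipe with an interp movement path built from start and end locations in its construction script.
; A looping timer checks the player controller's SpawnGateState: while true, it disables click events and moves balls from the remaining supply into a queue shown in the UI.
; Otherwise it spawns one queued BP_Ball per tick with a sound, forcing the state false while spawning.
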(event `self.ReceiveBeginPlay`
  (`self.BallSpawnTimer`))

(event `BallSpawnTimer`
  (bind _asbp_player_controller (cast `/Game/_Game/_Core/GameElement/Player/BP_PlayerController` (`GameplayStatics.GetPlayerController` 0)))
  (set `self.As BP Player Controller` _asbp_player_controller)
  (`KismetSystemLibrary.K2_SetTimerDelegate` (delegate `BallSpawn`) (`self.SpawnDelay`) true))

(event `BallSpawn`
  (if (> (`self.SpawningBalls`) 0)
    (set `/Game/_Game/_Core/GameElement/Player/BP_PlayerController.SpawnGateState` false (`self.As BP Player Controller`)))
  (if (`/Game/_Game/_Core/GameElement/Player/BP_PlayerController.SpawnGateState` (`self.As BP Player Controller`))
    (set `PlayerController.bEnableClickEvents` false (`self.As BP Player Controller`))
    (`|ExecutionSequence`
      (:`then_0`
        (goto _label :!via `Open`))
      (:`then_1`
        (`/Engine/EditorBlueprintResources/StandardMacros.Gate` true :!label _label
          (:`Exit`
            (bind _output_get (set `self.RemainingBalls` (`KismetMathLibrary.Clamp` (- (`self.RemainingBalls`) (`self.BallFlowrate`)) 0 101)))
            (if (not (<= _output_get 0))
              ;[1 1 1] Defini la variable SpawnQueue pour le spawn
              (`|ExecutionSequence`
                (:`then_0`
                  (set `self.BallSpawnQueue` (+ (`self.BallSpawnQueue`) (`self.BallFlowrate`)))
                  ;[1 1 1] Update la variable sur le player controller pour l'UI
                  (set `/Game/_Game/_Core/GameElement/Player/BP_PlayerController.BallsTotal` (`self.BallSpawnQueue`) (`self.As BP Player Controller`)))
                (:`then_1`
                  (`KismetSystemLibrary.PrintString` (`KismetStringLibrary.Concat_StrStr` "Spawn Queue : " (`KismetStringLibrary.Conv_IntToString` (`self.BallSpawnQueue`)))))
                (:`then_2`
                  (`KismetSystemLibrary.PrintString` (`KismetStringLibrary.Concat_StrStr` "Remaining Balls : " (`KismetStringLibrary.Conv_IntToString` (`self.RemainingBalls`)))))))))))
    (else
      (`|ExecutionSequence`
        (:`then_0`
          (goto _label :!via `Close`))
        (:`then_1`
          ;[1 1 1] Spawn les boules en fonction de la var BallSpawnQueue
          (set `self.SpawningBalls` (`self.BallSpawnQueue`))
          (if (> (`self.BallSpawnQueue`) 0)
            (bind _result (`/Engine/EditorBlueprintResources/StandardMacros.DecrementInt` (`self.BallSpawnQueue`))
              (:`  `
                (set `self.BallSpawnQueue` _result)
                (bind _result_2 (`/Engine/EditorBlueprintResources/StandardMacros.DecrementInt` (`self.SpawningBalls`))
                  (:`  `
                    (set `self.SpawningBalls` _result_2)
                    (`|SpawnActorFromClass` "/Game/_Game/_Core/GameElement/BP_Ball.BP_Ball_C" (`KismetMathLibrary.Conv_VectorToTransform` (`SceneComponent.K2_GetComponentLocation` (`self.SpawnerVolume`))) "Undefined" "MultiplyWithRoot" null null)
                    (`GameplayStatics.SpawnSound2D` "/Game/Sounds/Pipe_Exit_Cue.Pipe_Exit_Cue" 1.0 1.0 0.0 null)))))))))))

(fn `UserConstructionScript`
  (bind _interptomovement (`self.InterpToMovement`))
  (set `InterpToMovementComponent.ControlPoints` (`|MakeArray` (make `InterpControlPoint` (`self.StartLocation`)) (make `InterpControlPoint` (`self.EndLocation`))) _interptomovement)
  (set `InterpToMovementComponent.Duration` (`self.Duration`) _interptomovement))