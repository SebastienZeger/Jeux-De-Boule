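; BP_Seau is the bucket that collects colored balls and tallies them by color.
; When an actor tagged Ball overlaps the Deleto component, it destroys the ball and plays a water drop sound.
; FCheckColor compares the overlapping component's first material against eight color materials to set StateColor, which selects the matching score counter to increment on BP_GameMode.
; An unrecognized material leaves StateColor at its previous value.
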(event `self.Deleto.OnComponentBeginOverlap`
  (params (OverlappedComponent :type "PrimitiveComponent Object Reference") (OtherActor :type "Actor Object Reference") (OtherComp :type "PrimitiveComponent Object Reference") (OtherBodyIndex :type Integer) (bFromSweep :type Boolean) (SweepResult :type "HitResult Structure (by ref)"))
  (bind _gamemode (`self.GameMode`))
  (bind _gamemode_2 (`self.GameMode`))
  (if (`self.ActorHasTag` OtherActor "Ball")
    (`self.f_CheckColor` (`PrimitiveComponent.GetMaterial` OtherComp 0))
    (`self.K2_DestroyActor` OtherActor)
    (`GameplayStatics.SpawnSound2D` "/Game/Sounds/Water_Drop_Cue.Water_Drop_Cue" 1.0 1.0 0.0 null)
    (bind _asbp_game_mode (cast `/Game/_Game/_Core/GameElement/BP_GameMode` (`GameplayStatics.GetGameMode`)))
    (set `self.GameMode` _asbp_game_mode)
    (switch `/Game/_Game/_Core/GameElement/E_ColorBall` (`self.StateColor`)
      (:`NewEnumerator0`
        (bind _result (`/Engine/EditorBlueprintResources/StandardMacros.IncrementInt` (`/Game/_Game/_Core/GameElement/BP_GameMode.ScoreRed` _gamemode))
          (:`  `
            (set `/Game/_Game/_Core/GameElement/BP_GameMode.ScoreRed` _result _gamemode_2))))
      (:`NewEnumerator1`
        (bind _result_2 (`/Engine/EditorBlueprintResources/StandardMacros.IncrementInt` (`/Game/_Game/_Core/GameElement/BP_GameMode.ScoreYellow` _gamemode))
          (:`  `
            (set `/Game/_Game/_Core/GameElement/BP_GameMode.ScoreYellow` _result_2 _gamemode_2))))
      (:`NewEnumerator2`
        (bind _result_3 (`/Engine/EditorBlueprintResources/StandardMacros.IncrementInt` (`/Game/_Game/_Core/GameElement/BP_GameMode.ScoreBlue` _gamemode))
          (:`  `
            (set `/Game/_Game/_Core/GameElement/BP_GameMode.ScoreBlue` _result_3 _gamemode_2))))
      (:`NewEnumerator3`
        (bind _result_4 (`/Engine/EditorBlueprintResources/StandardMacros.IncrementInt` (`/Game/_Game/_Core/GameElement/BP_GameMode.ScoreOrange` _gamemode))
          (:`  `
            (set `/Game/_Game/_Core/GameElement/BP_GameMode.ScoreOrange` _result_4 _gamemode_2))))
      (:`NewEnumerator4`
        (bind _result_5 (`/Engine/EditorBlueprintResources/StandardMacros.IncrementInt` (`/Game/_Game/_Core/GameElement/BP_GameMode.ScoreGreen` _gamemode))
          (:`  `
            (set `/Game/_Game/_Core/GameElement/BP_GameMode.ScoreGreen` _result_5 _gamemode_2))))
      (:`NewEnumerator5`
        (bind _result_6 (`/Engine/EditorBlueprintResources/StandardMacros.IncrementInt` (`/Game/_Game/_Core/GameElement/BP_GameMode.ScorePurple` _gamemode))
          (:`  `
            (set `/Game/_Game/_Core/GameElement/BP_GameMode.ScorePurple` _result_6 _gamemode_2))))
      (:`NewEnumerator6`
        (bind _result_7 (`/Engine/EditorBlueprintResources/StandardMacros.IncrementInt` (`/Game/_Game/_Core/GameElement/BP_GameMode.ScoreWhite` _gamemode))
          (:`  `
            (set `/Game/_Game/_Core/GameElement/BP_GameMode.ScoreWhite` _result_7 _gamemode_2))))
      (:`NewEnumerator7`
        (bind _result_8 (`/Engine/EditorBlueprintResources/StandardMacros.IncrementInt` (`/Game/_Game/_Core/GameElement/BP_GameMode.ScoreBlack` _gamemode))
          (:`  `
            (set `/Game/_Game/_Core/GameElement/BP_GameMode.ScoreBlack` _result_8 _gamemode_2)))))))

(fn `f_CheckColor`
  (params (Material :type "MaterialInterface Object Reference"))
  (if (== Material "/Game/_Game/Material/M_Blue.M_Blue")
    (set `self.StateColor` "NewEnumerator2")
    (elif (== Material "/Game/_Game/Material/M_Yellow.M_Yellow")
      (set `self.StateColor` "NewEnumerator1")
      (elif (== Material "/Game/_Game/Material/M_Red.M_Red")
        (set `self.StateColor` "NewEnumerator0")
        (elif (== Material "/Game/_Game/Material/M_Orange.M_Orange")
          (set `self.StateColor` "NewEnumerator3")
          (elif (== Material "/Game/_Game/Material/M_Green.M_Green")
            (set `self.StateColor` "NewEnumerator4")
            (elif (== Material "/Game/_Game/Material/M_Purple.M_Purple")
              (set `self.StateColor` "NewEnumerator5")
              (elif (== Material "/Game/_Game/Material/M_White.M_White")
                (set `self.StateColor` "NewEnumerator6")
                (elif (== Material "/Game/_Game/Material/M_Black.M_Black")
                  (set `self.StateColor` "NewEnumerator7"))))))))))

(fn `UserConstructionScript`)