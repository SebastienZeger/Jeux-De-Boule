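; BP_Ball is a colored ball actor that mixes primary colors when it collides with another actor tagged "Ball".
; On a sphere hit, FColorMerge compares both materials and sets StateColorBall to purple, orange or green for red, blue and yellow pairs.
; After a tiny delay, the sphere swaps to the matching secondary material.
; FCheckMaterial maps a material to its color state but is not called within this Blueprint.
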(event `self.Sphere.OnComponentHit`
  (params (HitComponent :type "PrimitiveComponent Object Reference") (OtherActor :type "Actor Object Reference") (OtherComp :type "PrimitiveComponent Object Reference") (NormalImpulse :type "Vector Structure") (Hit :type "HitResult Structure (by ref)"))
  (bind (_bblockinghit _binitialoverlap _time _distance _location _impactpoint _normal _impactnormal _physmat _hitactor _hitcomponent) (`GameplayStatics.BreakHitResult` Hit))
  (bind _sphere (`self.Sphere`))
  (if (`self.ActorHasTag` _hitactor "Ball")
    (bind _output_get (set `self.MaterialHit` (`PrimitiveComponent.GetMaterial` _hitcomponent 0)))
    (`self.f_ColorMerge` _output_get (`PrimitiveComponent.GetMaterial` (`self.Sphere`) 0))
    (`KismetSystemLibrary.Delay` 0.001)
    (switch `/Game/_Game/_Core/GameElement/E_ColorBall` (`self.StateColorBall`)
      (:`NewEnumerator3`
        (`PrimitiveComponent.SetMaterial` _sphere 0 "/Game/_Game/Material/M_Orange.M_Orange"))
      (:`NewEnumerator4`
        (`PrimitiveComponent.SetMaterial` _sphere 0 "/Game/_Game/Material/M_Green.M_Green"))
      (:`NewEnumerator5`
        (`PrimitiveComponent.SetMaterial` _sphere 0 "/Game/_Game/Material/M_Purple.M_Purple")))))

(fn `f_Check Material`
  (params (Material :type "MaterialInterface Object Reference"))
  (if (== Material "/Game/_Game/Material/M_Blue.M_Blue")
    (set `self.StateColorBall` "NewEnumerator2")
    (elif (== Material "/Game/_Game/Material/M_Yellow.M_Yellow")
      (set `self.StateColorBall` "NewEnumerator1")
      (elif (== Material "/Game/_Game/Material/M_Red.M_Red")
        (set `self.StateColorBall` "NewEnumerator0")
        (elif (== Material "/Game/_Game/Material/M_Orange.M_Orange")
          (set `self.StateColorBall` "NewEnumerator3")
          (elif (== Material "/Game/_Game/Material/M_Green.M_Green")
            (set `self.StateColorBall` "NewEnumerator4")
            (elif (== Material "/Game/_Game/Material/M_Purple.M_Purple")
              (set `self.StateColorBall` "NewEnumerator5")
              (elif (== Material "/Game/_Game/Material/M_White.M_White")
                (set `self.StateColorBall` "NewEnumerator6")
                (elif (== Material "/Game/_Game/Material/M_Black.M_Black")
                  (set `self.StateColorBall` "NewEnumerator7"))))))))))

(fn `f_ColorMerge`
  (params (HitMaterial :type "MaterialInterface Object Reference") (SphereMaterial :type "MaterialInterface Object Reference"))
  (if (and (== HitMaterial "/Game/_Game/Material/M_Red.M_Red") (== SphereMaterial "/Game/_Game/Material/M_Blue.M_Blue"))
    (set `self.StateColorBall` "NewEnumerator5")
    (elif (and (== HitMaterial "/Game/_Game/Material/M_Red.M_Red") (== SphereMaterial "/Game/_Game/Material/M_Yellow.M_Yellow"))
      (set `self.StateColorBall` "NewEnumerator3")
      (elif (and (== HitMaterial "/Game/_Game/Material/M_Blue.M_Blue") (== SphereMaterial "/Game/_Game/Material/M_Yellow.M_Yellow"))
        (set `self.StateColorBall` "NewEnumerator4")
        (elif (and (== SphereMaterial "/Game/_Game/Material/M_Red.M_Red") (== HitMaterial "/Game/_Game/Material/M_Blue.M_Blue"))
          (set `self.StateColorBall` "NewEnumerator5")
          (elif (and (== SphereMaterial "/Game/_Game/Material/M_Red.M_Red") (== HitMaterial "/Game/_Game/Material/M_Yellow.M_Yellow"))
            (set `self.StateColorBall` "NewEnumerator3")
            (elif (and (== SphereMaterial "/Game/_Game/Material/M_Blue.M_Blue") (== HitMaterial "/Game/_Game/Material/M_Yellow.M_Yellow"))
              (set `self.StateColorBall` "NewEnumerator4"))))))))

(fn `UserConstructionScript`)