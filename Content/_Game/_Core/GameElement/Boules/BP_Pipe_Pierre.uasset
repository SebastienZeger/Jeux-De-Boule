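; BP_Pipe_Pierre is a ball-dispensing pipe that moves between start and end points set through InterpToMovement in the construction script.
; A looping timer checks the player controller's SpawnGateState: when true, it disables click events and moves batches of five from BallAmountToPlay into BallsToSpawn.
; Otherwise it spawns queued BP_Ball actors at the Arrow, one per tick, forcing the gate state false while SpawningBalls is positive.
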(event `self.ReceiveBeginPlay`
  (`|ExecutionSequence`
    (:`then_0`
      (`self.BallSpawnTimer`))))

(event `SpawnActor`)

(event `BallSpawnTimer`
  (`KismetSystemLibrary.K2_SetTimerDelegate` (delegate `BallSpawn`) 0.3 true))

(event `BallSpawn`
  (bind _asbp_player_controller (cast `/Game/_Game/_Core/GameElement/Player/BP_PlayerController` (`GameplayStatics.GetPlayerController` 0)))
  (set `self.As BP Player Controller` _asbp_player_controller)
  (if (> (`self.SpawningBalls`) 0)
    (set `/Game/_Game/_Core/GameElement/Player/BP_PlayerController.SpawnGateState` false (`self.As BP Player Controller`)))
  (if (`/Game/_Game/_Core/GameElement/Player/BP_PlayerController.SpawnGateState` (`self.As BP Player Controller`))
    (set `PlayerController.bEnableClickEvents` false (`self.As BP Player Controller`))
    (`|ExecutionSequence`
      (:`then_0`
        (goto _label :!via `Open`))
      (:`then_1`
        (`/Engine/EditorBlueprintResources/StandardMacros.Gate` true :!label _label
          (:`Exit`
            (bind _output_get (set `self.BallAmountToPlay` (`KismetMathLibrary.Clamp` (- (`self.BallAmountToPlay`) 5) 0 101)))
            (if (not (<= _output_get 0))
              (bind _output_get_2 (set `self.BallsToSpawn` (+ (`self.BallsToSpawn`) 5)))
              (`KismetSystemLibrary.PrintString` (`KismetStringLibrary.Conv_IntToString` _output_get_2))
              (`KismetSystemLibrary.PrintString` (`KismetStringLibrary.Conv_IntToString` (`self.BallAmountToPlay`))))))))
    (else
      (`|ExecutionSequence`
        (:`then_0`
          (goto _label :!via `Close`))
        (:`then_1`
          (set `self.SpawningBalls` (`self.BallsToSpawn`))
          (if (> (`self.BallsToSpawn`) 0)
            (bind _result (`/Engine/EditorBlueprintResources/StandardMacros.DecrementInt` (`self.BallsToSpawn`))
              (:`  `
                (set `self.BallsToSpawn` _result)
                (bind _result_2 (`/Engine/EditorBlueprintResources/StandardMacros.DecrementInt` (`self.SpawningBalls`))
                  (:`  `
                    (set `self.SpawningBalls` _result_2)
                    (`|SpawnActorFromClass` "/Game/_Game/_Core/GameElement/BP_Ball.BP_Ball_C" (`KismetMathLibrary.Conv_VectorToTransform` (`SceneComponent.K2_GetComponentLocation` (`self.Arrow`))) "Undefined" "MultiplyWithRoot" null null)
                    (`KismetSystemLibrary.Delay` 0.15)))))))))))

(fn `UserConstructionScript`
  (bind _interptomovement (`self.InterpToMovement`))
  (set `InterpToMovementComponent.ControlPoints` (`|MakeArray` (make `InterpControlPoint` (`self.StartLocation`)) (make `InterpControlPoint` (`self.EndLocation`))) _interptomovement)
  (set `InterpToMovementComponent.Duration` (`self.Duration`) _interptomovement))