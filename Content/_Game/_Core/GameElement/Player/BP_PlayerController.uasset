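; Player controller that moves the controlled BP_Seau pawn sideways through Enhanced Input or touch.
; The movement action feeds movement input along the pawn's right vector, while holding a touch opens a Tick gate that snaps its Y to the visibility trace hit under the finger.
; The spawn action toggles SpawnGateState while held, and BeginPlay requests a mapping rebuild for IMC_Seau.
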(event `EnhancedInput|/Game/_Game/_Core/GameElement/Inputs/IA_Seau_Movement`
  (params (ActionValue :type "Float (double-precision)") (ElapsedSeconds :type "Float (double-precision)") (TriggeredSeconds :type "Float (double-precision)") (InputAction :type "InputAction Object Reference" :default "/Game/_Game/_Core/GameElement/Inputs/IA_Seau_Movement.IA_Seau_Movement"))
  (:`Triggered`
    (bind _asbp_seau (cast `/Game/_Game/_Core/GameElement/Player/BP_Seau` (`self.K2_GetPawn`)))
    (`Pawn.AddMovementInput` _asbp_seau (`self.GetActorRightVector` _asbp_seau) ActionValue false)))

(event `self.ReceiveTick`
  (params (DeltaSeconds :type "Float (single-precision)"))
  (`/Engine/EditorBlueprintResources/StandardMacros.Gate` true :!label _label
    (:`Exit`
      (bind _asbp_seau (cast `/Game/_Game/_Core/GameElement/Player/BP_Seau` (`self.K2_GetPawn`)))
      (bind (_returnvalue_x _returnvalue_y _returnvalue_z) (`KismetMathLibrary.BreakVector` (`self.K2_GetActorLocation` _asbp_seau)))
      (`self.K2_SetActorLocation` _asbp_seau (`KismetMathLibrary.MakeVector` _returnvalue_x (.y (`.ImpactPoint` (`GameplayStatics.BreakHitResult` (`self.GetHitResultUnderFingerByChannel` (stale `InputTouch` FingerIndex) "TraceTypeQuery1")))) _returnvalue_z) false false))))

(event `InputTouch`
  (params (Location :type "Vector Structure") (FingerIndex :type "ETouchIndex Enum"))
  (:`Pressed`
    (goto _label :!via `Open`))
  (:`Released`
    (goto _label :!via `Close`)))

(event `self.ReceiveBeginPlay`
  (`EnhancedInputLibrary.RequestRebuildControlMappingsUsingContext` "/Game/_Game/_Core/GameElement/Inputs/IMC_Seau.IMC_Seau"))

(event `EnhancedInput|/Game/_Game/_Core/GameElement/Inputs/IA_Spawn`
  (params (ActionValue :type Boolean) (ElapsedSeconds :type "Float (double-precision)") (TriggeredSeconds :type "Float (double-precision)") (InputAction :type "InputAction Object Reference" :default "/Game/_Game/_Core/GameElement/Inputs/IA_Spawn.IA_Spawn"))
  (:`Started`
    (set `self.SpawnGateState` true))
  (:`Completed`
    (set `self.SpawnGateState` false)))

(fn `UserConstructionScript`)